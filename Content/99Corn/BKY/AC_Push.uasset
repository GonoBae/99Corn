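; Actor component that gives a BP_BasePerson a push attack, knocking another person away.
; BeginPush sphere-traces forward using the owner's BasicAttackStat distance and radius, with debug drawing, and stores a hit person as the target.
; RepPush, a replicated event, launches the target away from the owner at a speed inversely proportional to its Weight.
; EndPush sends a zero, non-overriding launch; stun-named leftovers suggest copying from a stun component.
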(event EventBeginPlay
  (CallFunction|InitializeStunComp))

(event EventTick
  (params (DeltaSeconds :type Float%20%28single-precision%29)))

(event Custom|Rep%20Push
  (params (Target :type BP%20Base%20Person%20Object%20Reference) (Velocity :type Vector))
  (Character|LaunchCharacter Target Velocity false false))

(fn BeginPush
  (bind _person (Variables|Default|Getperson))
  (bind _returnvalue (Transformation|GetActorLocation _person))
  (bind _basicattackstat (Variables|/Game/99Corn/BKY/BP_BasePerson.BP_BasePerson_C|GetBasicAttackStat _person))
  (Development|PrintString "Begin Push")
  (bind (_outhit _returnvalue_2) (Collision|SphereTraceByChannel _returnvalue (+ _returnvalue (* (Transformation|GetActorForwardVector _person) (Variables|/Game/99Corn/BKY/BP_BasicAttack.BP_BasicAttack_C|GetBasicDist _basicattackstat))) (Variables|/Game/99Corn/BKY/BP_BasicAttack.BP_BasicAttack_C|GetBasicRadius _basicattackstat) "TraceTypeQuery1" false 0 "ForDuration" true "(R=0.000000,G=0.047143,B=1.000000,A=1.000000)"))
  (if _returnvalue_2
    (bind _asbp_base_person (Utilities|Casting|CastToBP_BasePerson (.HitActor (Collision|BreakHitResult _outhit))))
    (bind _output_get (Variables|Default|Settargetperson _asbp_base_person))
    (CallFunction|RepPush (Variables|Default|Gettargetperson) (/ (* (Math|Vector|Normalize (- (Transformation|GetActorLocation _output_get) (Transformation|GetActorLocation (Variables|Default|Getperson)))) 1e+04) (Variables|/Game/99Corn/BKY/BP_BasicAttack.BP_BasicAttack_C|GetWeight (Variables|/Game/99Corn/BKY/BP_BasePerson.BP_BasePerson_C|GetBasicAttackStat _output_get))))))

(fn EndPush
  (Development|PrintString "End Stun")
  (CallFunction|RepPush (Variables|Default|Gettargetperson) "0, 0, 0"))

(fn InitializeStunComp
  (bind _asbp_base_person (Utilities|Casting|CastToBP_BasePerson (Components|GetOwner)))
  (Variables|Default|Setperson _asbp_base_person))