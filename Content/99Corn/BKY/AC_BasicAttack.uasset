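; Actor component that handles a basic attack for its owning BP_BasePerson, cached at BeginPlay.
; BeginAttack runs a debug-drawn forward sphere trace on the Visibility channel, using the owner's BasicAttackStat distance and radius.
; When it hits another BP_BasePerson, it stores the target and increments the owner's CurrentStack, without applying damage.
; EndAttack only prints "End Stun"; it and InitializeStunComp carry stun naming.
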(event EventBeginPlay
  (CallFunction|InitializeStunComp))

(event EventTick
  (params (DeltaSeconds :type Float%20%28single-precision%29)))

(fn BeginAttack
  (bind _person (Variables|Default|Getperson))
  (bind _person_2 (Variables|Default|Getperson))
  (bind _returnvalue (Transformation|GetActorLocation _person_2))
  (bind _basicattackstat (Variables|/Game/99Corn/BKY/BP_BasePerson.BP_BasePerson_C|GetBasicAttackStat _person_2))
  (Development|PrintString "Begin Attack")
  (bind (_outhit _returnvalue_2) (Collision|SphereTraceByChannel _returnvalue (+ _returnvalue (* (Transformation|GetActorForwardVector _person_2) (Variables|/Game/99Corn/BKY/BP_BasicAttack.BP_BasicAttack_C|GetBasicDist _basicattackstat))) (Variables|/Game/99Corn/BKY/BP_BasicAttack.BP_BasicAttack_C|GetBasicRadius _basicattackstat) "TraceTypeQuery1" false 0 "ForDuration"))
  (if _returnvalue_2
    (bind _asbp_base_person (Utilities|Casting|CastToBP_BasePerson (.HitActor (Collision|BreakHitResult _outhit))))
    (Variables|Default|Settargetperson _asbp_base_person)
    (bind _output_get (Variables|/Game/99Corn/BKY/BP_BasePerson.BP_BasePerson_C|SetCurrentStack _person (+ (Variables|/Game/99Corn/BKY/BP_BasePerson.BP_BasePerson_C|GetCurrentStack _person) 1)))
    (Development|PrintString (Utilities|String|Append "Basic Attack" (Utilities|String|ToString(Integer) _output_get)))))

(fn EndAttack
  (Development|PrintString "End Stun"))

(fn InitializeStunComp
  (bind _asbp_base_person (Utilities|Casting|CastToBP_BasePerson (Components|GetOwner)))
  (Variables|Default|Setperson _asbp_base_person))