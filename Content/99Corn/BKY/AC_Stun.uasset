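; AC_Stun is an actor component that lets its owning BP_BasePerson stun another person in front of it.
; BeginStun sphere-traces forward using the owner's BasicAttackStat range and radius, stores the hit person and sets its IsStunned flag through the RepStun event.
; A timer based on the attack's Duration calls EndStun to clear that flag on the single stored target.
; Debug prints and trace drawing remain enabled.
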(event EventBeginPlay
  (CallFunction|InitializeStunComp))

(event EventTick
  (params (DeltaSeconds :type Float%20%28single-precision%29)))

(event Custom|Rep%20Stun
  (params (IsStunned :type Boolean) (Target :type BP%20Base%20Person%20Object%20Reference))
  (Variables|/Script/Corn99.Corn99Character|SetIsStunned Target IsStunned)
  (if (not IsStunned)
    _))

(fn BeginStun
  (bind _person (Variables|Default|Getperson))
  (bind _returnvalue (Transformation|GetActorLocation _person))
  (bind _basicattackstat (Variables|/Game/99Corn/BKY/BP_BasePerson.BP_BasePerson_C|GetBasicAttackStat _person))
  (Development|PrintString "Begin Stun")
  (bind (_outhit _returnvalue_2) (Collision|SphereTraceByChannel _returnvalue (+ _returnvalue (* (Transformation|GetActorForwardVector _person) (Variables|/Game/99Corn/BKY/BP_BasicAttack.BP_BasicAttack_C|GetBasicDist _basicattackstat))) (Variables|/Game/99Corn/BKY/BP_BasicAttack.BP_BasicAttack_C|GetBasicRadius _basicattackstat) "TraceTypeQuery1" false 0 "ForDuration" true "(R=0.000000,G=0.047143,B=1.000000,A=1.000000)"))
  (if _returnvalue_2
    (bind _asbp_base_person (Utilities|Casting|CastToBP_BasePerson (.HitActor (Collision|BreakHitResult _outhit))))
    (bind _output_get (Variables|Default|Settargetperson _asbp_base_person))
    (CallFunction|RepStun true _output_get)
    (Utilities|Time|SetTimerbyFunctionName 0 "EndStun" (Variables|/Game/99Corn/BKY/BP_BasicAttack.BP_BasicAttack_C|GetDuration (Variables|/Game/99Corn/BKY/BP_BasePerson.BP_BasePerson_C|GetBasicAttackStat (Variables|Default|Getperson))))))

(fn EndStun
  (Development|PrintString "End Stun")
  (CallFunction|RepStun false (Variables|Default|Gettargetperson)))

(fn InitializeStunComp
  (bind _asbp_base_person (Utilities|Casting|CastToBP_BasePerson (Components|GetOwner)))
  (Variables|Default|Setperson _asbp_base_person))