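; BP_Person_BKY_BIG is a character Blueprint with a follow camera whose basic attack starts a push through ACPush.
; Each tick it writes its location to the MPC_Player material parameter collection.
; It also capsule-traces from the camera to itself on Visibility and sets the collection's Trace scalar to flag a hit, feeding materials that read it.
; The trace still draws debug shapes and prints the hit actor every frame.
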(event EventBeginPlay)

(event Collision|EventActorBeginOverlap
  (params (OtherActor :type Actor%20Object%20Reference)))

(event EventTick
  (params (DeltaSeconds :type Float%20%28single-precision%29))
  (bind _returnvalue (Transformation|GetActorLocation))
  (Rendering|Material|SetVectorParameterValue "/Game/99Corn/BKY/MPC_Player.MPC_Player" "PlayerLocation" (Math|Color|MakeColor (.x _returnvalue) (.y _returnvalue) (.z _returnvalue)) :!class /Script/Engine.KismetMaterialLibrary)
  (bind (_outhit _returnvalue_2) (Collision|CapsuleTraceByChannel (Transformation|GetWorldLocation (Variables|Default|GetFollowCamera)) (Transformation|GetActorLocation) 1.0 5e+01 "TraceTypeQuery1" false 0 "ForOneFrame"))
  (Development|PrintString (Utilities|GetDisplayName (.HitActor (Collision|BreakHitResult _outhit))))
  (if _returnvalue_2
    (Rendering|Material|SetScalarParameterValue "/Game/99Corn/BKY/MPC_Player.MPC_Player" "Trace" 1.0 :!class /Script/Engine.KismetMaterialLibrary)
    (else
      (Rendering|Material|SetScalarParameterValue "/Game/99Corn/BKY/MPC_Player.MPC_Player" "Trace" 0.0 :!class /Script/Engine.KismetMaterialLibrary))))

(fn ConstructionScript)

(fn BasicAttack
  (Default|BeginPush (Variables|Default|GetAC_Push)))