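; BP_WeaponTest is a test weapon actor that is picked up on overlap and can be thrown by the player.
; Overlap calls Pickup and an icon change, then binds UseWeapon to BP_ThirdPersonCharacter_CJH if that is the overlapping actor.
; UseWeapon enables physics on the Cube and calls ThrowWeaponTest.
; Comments mark the icon call for moving to the player and the use logic as needing revision.
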(event Custom|Use%20Weapon
  ;[1 1 1] 수정 필요
  (Physics|SetSimulatePhysics (Variables|Default|GetCube) true)
  (Class|PickupWeapon|ThrowWeaponTest))

(event EventBeginPlay)

(event Collision|EventActorBeginOverlap
  (params (OtherActor :type Actor%20Object%20Reference))
  (Class|PickupWeapon|Pickup OtherActor)
  (Default|CallChangeIcon "BP_WeaponTest") ; 코드에서 처리하는게 나을듯,플레이어에서 호출하도록 변경
  (bind _asbp_third_person_character_cjh (Utilities|Casting|CastToBP_ThirdPersonCharacter_CJH OtherActor))
  (bind _output_get (Variables|Default|SetPlayer _asbp_third_person_character_cjh))
  (EventDispatchers|BindEventtoUseWeapon _output_get (delegate Custom|Use%20Weapon)))

(event EventTick
  (params (DeltaSeconds :type Float%20%28single-precision%29)))

(fn ConstructionScript)