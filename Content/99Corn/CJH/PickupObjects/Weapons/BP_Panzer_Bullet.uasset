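; Projectile fired by the Panzer weapon that explodes on hit, firing a radial force impulse, explosion effect and debug spheres.
; An inner sphere overlap launches a third-person character hard away from the impact; if empty, a wider overlap applies a weaker launch.
; DoOnce limits each loop to one target, and the bullet then destroys itself.
; The outer launch direction reads the inner loop's cast result, not its own.
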(event OnComponentHit(Bullet)
  (params (HitComponent :type Primitive%20Component%20Object%20Reference) (OtherActor :type Actor%20Object%20Reference) (OtherComp :type Primitive%20Component%20Object%20Reference) (NormalImpulse :type Vector :default "0, 0, 0") (Hit :type Hit%20Result%20Structure%20%28by%20ref%29))
  (bind _location (Collision|BreakHitResult Hit))
  (Class|RadialForceComponent|FireImpulse (Variables|Default|GetRadialForce))
  (Effects|SpawnEmitteratLocation "/Game/StarterContent/Particles/P_Explosion.P_Explosion" _location)
  (Rendering|Debug|DrawDebugSphere _location 1e+02 12 "(R=0.000000,G=0.164614,B=1.000000,A=1.000000)" 4.0)
  (bind (_outactors _returnvalue) (Collision|SphereOverlapActors _location 1e+02 (Variables|Default|GetObject%20Types) "/Game/99Corn/CJH/BP_ThirdPersonCharacter_CJH.BP_ThirdPersonCharacter_CJH_C"))
  (for _array_element _outactors
    (Utilities|FlowControl|DoOnce false
      (:Completed
        (bind _asbp_third_person_character_cjh (Utilities|Casting|CastToBP_ThirdPersonCharacter_CJH _array_element))
        (Character|LaunchCharacter _asbp_third_person_character_cjh (* (Math|Vector|Normalize (+ (- (Transformation|GetActorLocation _asbp_third_person_character_cjh) _location) "10.000000,0.000000,1.000000")) 1e+03) false false)
        (Actor|DestroyActor))))
  (if _returnvalue ; 100내 처리
    _
    (else
      (Rendering|Debug|DrawDebugSphere _location 2.5e+02 12 "(R=0.406250,G=0.503990,B=1.000000,A=1.000000)" 4.0)
      (bind _outactors_2 (Collision|SphereOverlapActors _location 2.5e+02 (Variables|Default|GetObject%20Types) "/Game/99Corn/CJH/BP_ThirdPersonCharacter_CJH.BP_ThirdPersonCharacter_CJH_C"))
      (for _array_element_2 _outactors_2
        (Utilities|FlowControl|DoOnce false
          (:Completed
            (bind _asbp_third_person_character_cjh_2 (Utilities|Casting|CastToBP_ThirdPersonCharacter_CJH _array_element_2))
            (Character|LaunchCharacter _asbp_third_person_character_cjh_2 (* (Math|Vector|Normalize (+ (- (Transformation|GetActorLocation _asbp_third_person_character_cjh) _location) "10.000000,0.000000,1.000000")) 4e+02) false false)
            (Actor|DestroyActor))))))
  (Actor|DestroyActor))

(fn ConstructionScript)