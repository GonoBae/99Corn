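; BP_Panzer is a pickup weapon that fires BP_Panzer_Bullet projectiles in the player's view direction.
; On actor overlap it calls Pickup and rotates the mesh, then, for BP_ThirdPersonCharacter_CJH only, binds UseWeapon to the character and disables mesh collision.
; UseWeapon spawns a bullet at the Scene component's location with the camera's rotation.
; Tick constantly matches the mesh's world rotation to the camera, even before pickup, overriding the overlap rotation.
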(event Custom|Use%20Weapon
  (Game|SpawnActorfromClass "/Game/99Corn/CJH/PickupObjects/Weapons/BP_Panzer_Bullet.BP_Panzer_Bullet_C" (Math|Transform|MakeTransform (Transformation|GetWorldLocation (Variables|Default|GetScene)) (Camera|GetCameraRotation (Game|GetPlayerCameraManager 0))) "Undefined" "MultiplyWithRoot" 0 0))

(event EventBeginPlay)

(event Collision|EventActorBeginOverlap
  (params (OtherActor :type Actor%20Object%20Reference))
  (Class|PickupWeapon|Pickup OtherActor)
  (Transformation|AddRelativeRotation (Variables|Default|Getpanzer) "90.000000,0.000000,0.000000" false false)
  (bind _asbp_third_person_character_cjh (Utilities|Casting|CastToBP_ThirdPersonCharacter_CJH OtherActor))
  (bind _output_get (Variables|Default|SetPlayer _asbp_third_person_character_cjh))
  (EventDispatchers|BindEventtoUseWeapon _output_get (delegate Custom|Use%20Weapon))
  (Collision|SetCollisionEnabled (Variables|Default|Getpanzer) "NoCollision"))

(event EventTick
  (params (DeltaSeconds :type Float%20%28single-precision%29))
  (Transformation|SetWorldRotation (Variables|Default|Getpanzer) (Camera|GetCameraRotation (Game|GetPlayerCameraManager 0)) false false))

(fn ConstructionScript)