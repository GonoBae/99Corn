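; Fan weapon pickup that blows characters away in a cone along the wielder's camera direction.
; On overlap it runs Pickup, binds the character's use and release events, and refills DataAsset ammo.
; Use starts a fast looping timer, gated by IsUsingGun, that spends ammo per tick on a debug-drawn cone query from GunPoint.
; Hit characters are launched along the camera forward by Damage, doubled at close range.
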(event Custom|UseWaepon
  (bind _output_get (Variables|Default|SetisUsingGun true))
  (Utilities|Time|SetTimerbyEvent (delegate Custom|CustomEvent_0) 0.01 _output_get))

(event Custom|CustomEvent
  (Variables|Default|SetisUsingGun false))

(event Custom|CustomEvent_0
  (bind _dataasset (Variables|Default|GetDataAsset))
  (bind _closehitactors (Variables|Default|GetcloseHitActors))
  (bind _farhitactors (Variables|Default|GetfarHitActors))
  (bind _dataasset_2 (Variables|Default|GetDataAsset))
  (bind _damage (Variables|/Game/99Corn/CJH/PickupObjects/BP_WeaponDataAsset.BP_WeaponDataAsset_C|GetDamage _dataasset_2))
  (if (Variables|Default|GetisUsingGun)
    (if (> (Variables|/Game/99Corn/CJH/PickupObjects/BP_WeaponDataAsset.BP_WeaponDataAsset_C|GetAmmo (Variables|Default|GetDataAsset)) 0)
      (bind (_closerangeactors _farrangeactors) (Class|PickupWeapon|FindActorsinCone (Transformation|GetWorldLocation (Variables|/Game/99Corn/CJH/BP_ThirdPersonCharacter_CJH.BP_ThirdPersonCharacter_CJH_C|GetGunPoint (stale Collision|EventActorBeginOverlap _asbp_third_person_character_cjh))) (Math|Vector|GetForwardVector (Variables|/Script/Corn99.Corn99Character|GetFollowCamera (stale Collision|EventActorBeginOverlap _asbp_third_person_character_cjh))) 4e+01 5e+02 (Variables|Default|GetObject%20Types) (Variables|Default|GetIgnore%20Actors) true))
      ;[1 1 1] 근접 미지
      (for _array_element _closerangeactors
        (Utilities|Array|AddUnique _closehitactors _array_element))
      (for _array_element_2 _closehitactors
        (bind _asbp_third_person_character_cjh (Utilities|Casting|CastToBP_ThirdPersonCharacter_CJH _array_element_2))
        (Character|LaunchCharacter _asbp_third_person_character_cjh (* (Math|Vector|GetForwardVector (Variables|/Script/Corn99.Corn99Character|GetFollowCamera (stale Collision|EventActorBeginOverlap _asbp_third_person_character_cjh))) (* _damage 2.0)) false false))
      ;[1 1 1] 원거리 데미지
      (for _array_element_3 _farrangeactors
        (Utilities|Array|AddUnique _farhitactors _array_element_3))
      (for _array_element_4 _farhitactors
        (bind _asbp_third_person_character_cjh_2 (Utilities|Casting|CastToBP_ThirdPersonCharacter_CJH _array_element_4))
        (Character|LaunchCharacter _asbp_third_person_character_cjh_2 (* (Math|Vector|GetForwardVector (Variables|/Script/Corn99.Corn99Character|GetFollowCamera (stale Collision|EventActorBeginOverlap _asbp_third_person_character_cjh))) _damage) false false))
      ;[1 1 1] 리스트 비움
      (Utilities|Array|Clear (Variables|Default|GetcloseHitActors))
      (Utilities|Array|Clear (Variables|Default|GetfarHitActors))
      (Variables|/Game/99Corn/CJH/PickupObjects/BP_WeaponDataAsset.BP_WeaponDataAsset_C|SetAmmo _dataasset (- (Variables|/Game/99Corn/CJH/PickupObjects/BP_WeaponDataAsset.BP_WeaponDataAsset_C|GetAmmo _dataasset) 1)))))

(event Collision|EventActorBeginOverlap
  (params (OtherActor :type Actor%20Object%20Reference))
  (Class|PickupWeapon|Pickup OtherActor)
  (bind _asbp_third_person_character_cjh (Utilities|Casting|CastToBP_ThirdPersonCharacter_CJH OtherActor))
  (EventDispatchers|BindEventtoUseWeapon _asbp_third_person_character_cjh (delegate Custom|UseWaepon))
  (EventDispatchers|BindEventtoNotUsetWeapon _asbp_third_person_character_cjh (delegate Custom|CustomEvent))
  (Variables|/Game/99Corn/CJH/PickupObjects/BP_WeaponDataAsset.BP_WeaponDataAsset_C|SetAmmo (Variables|Default|GetDataAsset) 1000))

(fn ConstructionScript
  (bind _dataasset (Variables|Default|GetDataAsset)
    (:then
      (Variables|Default|SetDataAsset _dataasset))
    (:else)))