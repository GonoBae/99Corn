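; BP_WindGunTest is a prototype wind gun pickup that attaches to the overlapping third-person character's hand socket and binds to its use-weapon event.
; Using it fires three debug-drawn sphere traces from the gun point along the camera's forward vector, two with endpoints offset along world Y.
; The trace results currently go unused: the character-launch logic is disconnected, as is the data-driven mesh setup.
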(event Custom|UseWeapon
  (bind _outhit (Collision|SphereTraceForObjects (Transformation|GetWorldLocation (Variables|/Game/99Corn/CJH/BP_ThirdPersonCharacter_CJH.BP_ThirdPersonCharacter_CJH_C|GetGunPoint (stale Collision|EventActorBeginOverlap _output_get))) (+ (Transformation|GetWorldLocation (Variables|/Game/99Corn/CJH/BP_ThirdPersonCharacter_CJH.BP_ThirdPersonCharacter_CJH_C|GetGunPoint (stale Collision|EventActorBeginOverlap _output_get))) (* (Math|Vector|GetForwardVector (Variables|/Script/Corn99.Corn99Character|GetFollowCamera (stale Collision|EventActorBeginOverlap _output_get))) 1e+03)) 3e+01 (Variables|Default|GetObject%20Types) false 0 "ForDuration"))
  (Collision|SphereTraceForObjects (Transformation|GetWorldLocation (Variables|/Game/99Corn/CJH/BP_ThirdPersonCharacter_CJH.BP_ThirdPersonCharacter_CJH_C|GetGunPoint (stale Collision|EventActorBeginOverlap _output_get))) (+ (+ (Transformation|GetWorldLocation (Variables|/Game/99Corn/CJH/BP_ThirdPersonCharacter_CJH.BP_ThirdPersonCharacter_CJH_C|GetGunPoint (stale Collision|EventActorBeginOverlap _output_get))) (* (Math|Vector|GetForwardVector (Variables|/Script/Corn99.Corn99Character|GetFollowCamera (stale Collision|EventActorBeginOverlap _output_get))) 1e+03)) "0.000000,500.000000,0.000000") 3e+01 (Variables|Default|GetObject%20Types) false 0 "ForDuration")
  (Collision|SphereTraceForObjects (Transformation|GetWorldLocation (Variables|/Game/99Corn/CJH/BP_ThirdPersonCharacter_CJH.BP_ThirdPersonCharacter_CJH_C|GetGunPoint (stale Collision|EventActorBeginOverlap _output_get))) (+ (+ (Transformation|GetWorldLocation (Variables|/Game/99Corn/CJH/BP_ThirdPersonCharacter_CJH.BP_ThirdPersonCharacter_CJH_C|GetGunPoint (stale Collision|EventActorBeginOverlap _output_get))) (* (Math|Vector|GetForwardVector (Variables|/Script/Corn99.Corn99Character|GetFollowCamera (stale Collision|EventActorBeginOverlap _output_get))) 1e+03)) "0.000000,-500.000000,0.000000") 3e+01 (Variables|Default|GetObject%20Types) false 0 "ForDuration"))

(event Collision|EventActorBeginOverlap
  (params (OtherActor :type Actor%20Object%20Reference))
  (bind _asbp_third_person_character_cjh (Utilities|Casting|CastToBP_ThirdPersonCharacter_CJH OtherActor))
  (bind _output_get (Variables|Default|SetPlayer _asbp_third_person_character_cjh))
  (Transformation|AttachComponentToComponent (Variables|/Script/Engine.Character|GetMesh _output_get) "HandSocket" "KeepWorld" "KeepRelative" "KeepWorld" false)
  (EventDispatchers|BindEventtoUseWeapon _output_get (delegate Custom|UseWeapon)))

(fn ConstructionScript)